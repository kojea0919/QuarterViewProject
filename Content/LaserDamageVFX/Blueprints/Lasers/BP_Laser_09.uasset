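; BP_Laser_09 is a laser actor that fires a beam along its arrow and shows impact effects where it hits.
; Each tick it line-traces on Visibility up to LaserLength, then stretches the laser mesh to the hit distance and activates the flash.
; Hits spawn two emitters every frame, one aligned to the surface normal.
; BeginPlay clears the RT_Damage render target and creates an M_Brush dynamic material, but this graph never paints with them.
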(event EventBeginPlay
  ;[1 1 1] Create/Remove Brush
  (Rendering|ClearRenderTarget2D "/Game/LaserDamageVFX/RenderTargets/RT_Damage.RT_Damage")
  (bind _returnvalue (Rendering|Material|CreateDynamicMaterialInstance "/Game/LaserDamageVFX/Materials/M_Brush.M_Brush" "None" :!class /Script/Engine.KismetMaterialLibrary))
  (Variables|Default|SetBrush _returnvalue))

(event EventTick
  (params (DeltaSeconds :type Float%20%28single-precision%29))
  (bind _arrow (Variables|Default|GetArrow))
  (bind _returnvalue (Transformation|GetWorldLocation _arrow))
  ;[1 1 1] LineTrace
  (bind (_outhit _returnvalue_2) (Collision|LineTraceByChannel _returnvalue (+ _returnvalue (* (Math|Vector|GetForwardVector _arrow) (Variables|Default|GetLaserLength))) "TraceTypeQuery1" true 0 "None"))
  (if _returnvalue_2
    ;[1 1 1] SpawnLaserMesh
    (Transformation|SetWorldScale3D (Variables|Default|GetLaser) (Math|Vector|MakeVector 0.5 0.5 (/ (Math|Vector|Distance(Vector) (.Location (Collision|BreakHitResult _outhit)) (.TraceStart (Collision|BreakHitResult _outhit))) 19.5)))
    ;[1 1 1] SpawnHitParticle
    (Rendering|SetVisibility (Variables|Default|GetLaser) true false)
    (Components|Activation|SetActive (Variables|Default|GetFlash) true false)
    (Effects|SpawnEmitteratLocation "/Game/LaserDamageVFX/Particles/Hits/P_Hit_08.P_Hit_08" (.Location (Collision|BreakHitResult _outhit)))
    (Effects|SpawnEmitteratLocation "/Game/LaserDamageVFX/Particles/P_LaserImpact.P_LaserImpact" (+ (.Location (Collision|BreakHitResult _outhit)) (.ImpactNormal (Collision|BreakHitResult _outhit))) (Math|Conversions|RotationFromXVector (.ImpactNormal (Collision|BreakHitResult _outhit))))))

(fn ConstructionScript)