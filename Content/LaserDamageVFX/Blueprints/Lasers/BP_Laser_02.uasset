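; Laser actor that burns damage into surfaces it hits by painting into render targets at runtime.
; Each tick it line traces along its arrow, stretches the laser and beam to the hit, and spawns impact and melting particles.
; The first hit on each actor name creates a render target and dynamic material, then a brush material paints at the hit's collision UV.
; The UV squish sampling is never executed.
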(event EventBeginPlay
  ;[1 1 1] Create/Remove Brush
  (Rendering|ClearRenderTarget2D "/Game/LaserDamageVFX/RenderTargets/RT_Damage.RT_Damage")
  (bind _returnvalue (Rendering|Material|CreateDynamicMaterialInstance "/Game/LaserDamageVFX/Materials/M_Brush.M_Brush" "None" :!class /Script/Engine.KismetMaterialLibrary))
  (Variables|Default|SetBrush _returnvalue))

(event EventTick
  (params (DeltaSeconds :type Float%20%28single-precision%29))
  (bind _arrow (Variables|Default|GetArrow))
  (bind _beam (Variables|Default|GetBeam))
  (bind _returnvalue (Transformation|GetWorldLocation _arrow))
  ;[1 1 1] LineTrace
  (bind (_outhit _returnvalue_2) (Collision|LineTraceByChannel _returnvalue (+ _returnvalue (* (Math|Vector|GetForwardVector _arrow) (Variables|Default|GetLaserLength))) "TraceTypeQuery1" true 0 "None"))
  (if _returnvalue_2
    ;[1 1 1] SpawnLaserMesh
    (Transformation|SetWorldScale3D (Variables|Default|GetLaser) (Math|Vector|MakeVector 0.5 0.5 (/ (Math|Vector|Distance(Vector) (.Location (Collision|BreakHitResult _outhit)) (.TraceStart (Collision|BreakHitResult _outhit))) 19.5)))
    ;[1 1 1] SpawnHitParticle
    (Rendering|SetVisibility (Variables|Default|GetLaser) true false)
    (Components|Activation|SetActive (Variables|Default|GetFlash) true false)
    (Components|Activation|SetActive (Variables|Default|GetBeam) true false)
    (Class|ParticleSystemComponent|SetBeamSourcePoint _beam 0 (.TraceStart (Collision|BreakHitResult _outhit)))
    (Class|ParticleSystemComponent|SetBeamTargetPoint _beam 0 (.Location (Collision|BreakHitResult _outhit)))
    (Effects|SpawnEmitteratLocation "/Game/LaserDamageVFX/Particles/Hits/P_Hit_02.P_Hit_02" (.Location (Collision|BreakHitResult _outhit)))
    (Effects|SpawnEmitteratLocation "/Game/LaserDamageVFX/Particles/P_Melting_Green.P_Melting_Green" (.Location (Collision|BreakHitResult _outhit)))
    ;[1 1 1] LaserDamage
    (|CollapseGraph_0 (.HitComponent (Collision|BreakHitResult _outhit)) _outhit (.HitActor (Collision|BreakHitResult _outhit)) (.HitComponent (Collision|BreakHitResult _outhit)) (.HitComponent (Collision|BreakHitResult _outhit)) (.FaceIndex (Collision|BreakHitResult _outhit)) (.HitComponent (Collision|BreakHitResult _outhit)) (.FaceIndex (Collision|BreakHitResult _outhit)) (.Location (Collision|BreakHitResult _outhit)) (.Location (Collision|BreakHitResult _outhit)) (.Normal (Collision|BreakHitResult _outhit)) (.Normal (Collision|BreakHitResult _outhit)))))

(fn ConstructionScript)