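; Archer player Blueprint that drives an expandable radius effect, apparently black-and-white, through the MPC_BlackAndWhite material parameter collection.
; Tick writes the actor's location to the PlayerLocation parameter every frame.
; Holding O plays a timeline that feeds the Radius parameter and prints a debug string.
; Releasing O reverses that timeline at a faster play rate to shrink the radius.
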(event Custom|Reduce%20Radius
  (Components|Timeline|SetPlayRate (Variables|Default|GetBlackWhite_TL) 2.0)
  (bind _radius (Timeline|BlackWhite_TL Reverse)
    (:Update
      (Rendering|Material|SetScalarParameterValue "/Game/GamePlay/GamePlayEffect/BlackAndWhite/MPC_BlackAndWhite.MPC_BlackAndWhite" "Radius" _radius :!class /Script/Engine.KismetMaterialLibrary))))

(event Custom|Expand%20Radius
  (Components|Timeline|SetPlayRate (Variables|Default|GetBlackWhite_TL) 1.0)
  (bind _radius (Timeline|BlackWhite_TL Play)
    (:Update
      (Rendering|Material|SetScalarParameterValue "/Game/GamePlay/GamePlayEffect/BlackAndWhite/MPC_BlackAndWhite.MPC_BlackAndWhite" "Radius" _radius :!class /Script/Engine.KismetMaterialLibrary))))

(event EventBeginPlay)

(event Collision|EventActorBeginOverlap
  (params (OtherActor :type Actor%20Object%20Reference)))

(event EventTick
  (params (DeltaSeconds :type Float%20%28single-precision%29))
  (Rendering|Material|SetVectorParameterValue "/Game/GamePlay/GamePlayEffect/BlackAndWhite/MPC_BlackAndWhite.MPC_BlackAndWhite" "PlayerLocation" (Math|Conversions|ToLinearColor(Vector) (Transformation|GetActorLocation)) :!class /Script/Engine.KismetMaterialLibrary))

(event Input|KeyboardEvents|O
  (params (Key :type Key%20Structure :default "None"))
  (:Pressed
    (CallFunction|ExpandRadius)
    (Development|PrintString "Hello"))
  (:Released
    (CallFunction|ReduceRadius)))

(fn ConstructionScript)