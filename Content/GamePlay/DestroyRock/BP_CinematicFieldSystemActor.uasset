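; Chaos field system actor in the DestroyRock gameplay folder that fires a one-shot destruction field, named for cinematic use.
; On BeginPlay it applies a very strong external cluster strain through a radial falloff with no attenuation, sized and centered by its Sphere component.
; It then applies a radial linear velocity from the sphere's center, scaled by RadialFieldMagnitude, to push the pieces.
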(event EventBeginPlay
  (CallFunction|AddForcetoActor))

(event Collision|EventActorBeginOverlap
  (params (OtherActor :type Actor%20Object%20Reference)))

(event EventTick
  (params (DeltaSeconds :type Float%20%28single-precision%29)))

(fn ConstructionScript)

(fn AddForcetoActor
  (bind _fieldsystemcomponent (Variables|Default|GetFieldSystemComponent))
  (bind _sphere (Variables|Default|GetSphere))
  (bind _returnvalue (Transformation|GetWorldLocation _sphere))
  (Class|FieldSystemComponent|ApplyPhysicsField _fieldsystemcomponent true "Field_ExternalClusterStrain" 0 (Field|SetRadialFalloff (Variables|Default|GetRadialFalloff) 5e+05 0.0 1.0 0.0 (Components|Sphere|GetScaledSphereRadius _sphere) _returnvalue "Field_FallOff_None"))
  (Class|FieldSystemComponent|ApplyPhysicsField _fieldsystemcomponent true "Field_LinearVelocity" 0 (Field|SetRadialVector (Variables|Default|GetRadialVector) (Variables|Default|GetRadialFieldMagnitude) _returnvalue)))