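; BP_Phase3Plane is a cinematic prop for the boss phase 3 cinematics that fades a mesh's material opacity in and out.
; BeginPlay puts a dynamic material instance on the Cube component.
; StartCreate and StartRemove set flags, and Tick ramps the Opacity parameter linearly toward a partial maximum or zero, with removal taking priority.
; The final clamped value is never written to the material.
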(event EventBeginPlay
  (bind _returnvalue (Rendering|Material|CreateDynamicMaterialInstance (Rendering|Material|GetMaterial (Variables|Default|GetCube) 0) "None" "None" :!class /Script/Engine.KismetMaterialLibrary))
  (bind _output_get (Variables|Default|SetMaterial _returnvalue))
  (Rendering|Material|SetMaterial (Variables|Default|GetCube) 0 _output_get))

(event EventTick
  (params (DeltaSeconds :type Float%20%28single-precision%29))
  (if (Variables|Default|GetNeedRemove)
    (bind _output_get (Variables|Default|SetCurOpacity (- (Variables|Default|GetCurOpacity) (* DeltaSeconds 0.4))))
    (if (<= _output_get 0.0)
      (Variables|Default|SetNeedRemove false)
      (Variables|Default|SetCurOpacity 0.0)
      (else
        (Rendering|Material|SetScalarParameterValue (Variables|Default|GetMaterial) "Opacity" _output_get :!class /Script/Engine.MaterialInstanceDynamic)))
    (elif (Variables|Default|GetNeedCreate)
      (bind _output_get_2 (Variables|Default|SetCurOpacity (+ (* DeltaSeconds 0.4) (Variables|Default|GetCurOpacity))))
      (if (> _output_get_2 0.8)
        (Variables|Default|SetCurOpacity 0.8)
        (Variables|Default|SetNeedCreate false)
        (else
          (Rendering|Material|SetScalarParameterValue (Variables|Default|GetMaterial) "Opacity" _output_get_2 :!class /Script/Engine.MaterialInstanceDynamic))))))

(fn ConstructionScript)

(fn StartRemove
  (Variables|Default|SetNeedRemove true))

(fn StartCreate
  (Variables|Default|SetNeedCreate true))