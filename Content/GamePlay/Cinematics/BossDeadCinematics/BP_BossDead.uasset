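; Cinematic boss death actor that dissolves its mesh in two independently triggered stages, body and non-body.
; BeginPlay replaces every mesh material with a dynamic instance and caches it in an array.
; SetDissolveBody and SetDissolveWithoutBody raise flags that make Tick advance the "Dissolve" scalar at a fixed rate, on the two body slots or all others respectively.
; Each stage stops and resets its counter upon reaching full value.
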(event EventBeginPlay
  (for (_array_element _array_index) (Rendering|Material|GetMaterials (Variables|Character|GetMesh))
    (bind _returnvalue (Rendering|Material|CreateDynamicMaterialInstance _array_element "None" "None" :!class /Script/Engine.KismetMaterialLibrary))
    (Utilities|Array|Add (Variables|Default|GetDynMaterialArr) _returnvalue)
    (Rendering|Material|SetMaterial (Variables|Character|GetMesh) _array_index _returnvalue)))

(event EventTick
  (params (DeltaSeconds :type Float%20%28single-precision%29))
  (Utilities|FlowControl|Sequence
    (:then_0
      (if (Variables|Default|GetStartDissolveWithoutBody)
        (bind _output_get (Variables|Default|SetCurDissolveWithoutBody (+ (* DeltaSeconds 0.12) (Variables|Default|GetCurDissolveWithoutBody))))
        (if (>= _output_get 1.0)
          (Variables|Default|SetStartDissolveWithoutBody false)
          (Variables|Default|SetCurDissolveWithoutBody -0.5)
          (else
            (for (_array_element _array_index) (Variables|Default|GetDynMaterialArr)
              (if (not (or (== _array_index 2) (== _array_index 0)))
                (Rendering|Material|SetScalarParameterValue _array_element "Dissolve" (Variables|Default|GetCurDissolveWithoutBody) :!class /Script/Engine.MaterialInstanceDynamic)))))))
    (:then_1
      (if (Variables|Default|GetStartDissolveBody)
        (bind _output_get_2 (Variables|Default|SetCurDissolveBody (+ (* DeltaSeconds 0.12) (Variables|Default|GetCurDissolveBody))))
        (if (>= _output_get_2 1.0)
          (Variables|Default|SetStartDissolveBody false)
          (Variables|Default|SetCurDissolveBody -0.5)
          (else
            (Rendering|Material|SetScalarParameterValue (Utilities|Array|Get(acopy) (Variables|Default|GetDynMaterialArr) 2) "Dissolve" (Variables|Default|GetCurDissolveBody) :!class /Script/Engine.MaterialInstanceDynamic)
            (Rendering|Material|SetScalarParameterValue (Utilities|Array|Get(acopy) (Variables|Default|GetDynMaterialArr)) "Dissolve" (Variables|Default|GetCurDissolveBody) :!class /Script/Engine.MaterialInstanceDynamic)))))))

(fn ConstructionScript)

(fn SetDissolveBody
  (Variables|Default|SetStartDissolveBody true))

(fn SetDissolveWithoutBody
  (Variables|Default|SetStartDissolveWithoutBody true))